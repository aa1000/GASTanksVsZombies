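; Tank projectile Blueprint that adds an animated Paper2D explosion to its parent class's explode behavior.
; OnExplode plays a non-looping explosion flipbook, clears the projectile sprite and zeroes the projectile speed.
; The parent's OnExplode is deferred until the flipbook's finished-playing event fires, so the animation completes first.
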(event Custom|FinishedExploding
  (|CallParentFunction))

(event EventOnExplode
  (bind _explodeflipbook (Variables|Default|GetExplodeFlipBook))
  (Sprite|SetFlipbook _explodeflipbook (Variables|Default|GetExplosionFlipbook))
  (Audio|Components|Audio|Play _explodeflipbook)
  (Components|Timeline|SetLooping _explodeflipbook false)
  (EventDispatchers|BindEventtoOnFinishedPlaying _explodeflipbook (delegate Custom|FinishedExploding))
  (Rendering|Components|Sprite|SetSprite (Variables|Default|GetProjectileSprite) 0)
  (Variables|Default|SetProjectileSpeed 0.0))

(fn ConstructionScript)