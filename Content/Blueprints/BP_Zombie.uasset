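; BP_Zombie is an enemy actor that presents a green zombie's walk, attack and death with Paper2D flipbooks.
; Its walk event loops the walk flipbook and scales playback rate with movement speed, while attack plays its flipbook once from the start.
; On death it disables collision and tick, shows the dead flipbook with a squish sound, lowers it below live zombies, then calls the parent death logic after a delay.
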(event EventZombieWalk
  (params (DeltaSeconds :type Float%20%28single-precision%29) (DistanceWalkedThisFrame :type Vector%20%28by%20ref%29 :default "0, 0, 0"))
  (bind _returnvalue (Class|PawnwithAbilities|GetMoveSpeed))
  (bind _paperflipbook (Variables|Default|GetPaperFlipbook))
  ;[1 0.8635 0] play the zombie walk animation
  (Sprite|SetFlipbook _paperflipbook "/Game/Flipbooks/GreenZombieWalk.GreenZombieWalk")
  (Components|Timeline|SetLooping _paperflipbook true)
  (Audio|Components|Audio|Play _paperflipbook)
  (Components|Timeline|SetPlayRate _paperflipbook (Math|Float|MapRangeClamped (/ (Math|Vector|VectorLength DistanceWalkedThisFrame) DeltaSeconds) _returnvalue (* _returnvalue 2.0) 1.0 2.0)))

(event EventZombieAttack
  (params (DeltaSeconds :type Float%20%28single-precision%29))
  (bind _paperflipbook (Variables|Default|GetPaperFlipbook))
  ;[0.5635 0 0.000622] Zombie Attack
  (Sprite|SetFlipbook _paperflipbook "/Game/Flipbooks/GreenZombieAttack.GreenZombieAttack")
  (Components|Timeline|SetLooping _paperflipbook false)
  (Components|Timeline|PlayfromStart _paperflipbook)
  (Components|Timeline|SetPlayRate _paperflipbook 1.0))

(event EventOnDeath
  (bind _paperflipbook (Variables|Default|GetPaperFlipbook))
  ;[0 0.2219 0.003373] When the zombie dies change the texture then destroy the actor after 5 seconds
  (Collision|SetActorEnableCollision false)
  (Actor|Tick|SetActorTickEnabled false)
  (Sprite|SetFlipbook _paperflipbook "/Game/Flipbooks/ZombieDeadFlipbook.ZombieDeadFlipbook")
  (Components|Timeline|SetLooping _paperflipbook true)
  (Audio|PlaySound2D "/Game/Audio/SoundCues/SC_Squish.SC_Squish" 1.0 1.0 0.0 0 0)
  (Transformation|AddRelativeLocation (Variables|Default|GetPaperFlipbook) "0, 0,-5.000000" false false) ; move the zombie down so it doesn't block live zombies on Z
  (Utilities|FlowControl|Delay 5.0)
  (|CallParentFunction))

(fn ConstructionScript)